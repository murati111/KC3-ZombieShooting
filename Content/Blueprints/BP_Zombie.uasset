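; BP_Zombie is a zombie enemy character that hurts Player-tagged actors touching its sphere while it is alive.
; BeginPlay blends physics simulation below a named bone, and the construction script sets walk speed from Speed.
; When damage depletes Health, it ragdolls once, drops its capsule, increments ZombieGameMode's NumZombie and expires shortly after.
; Move-to-player and hit-stop logic are present but unconnected.
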(event OnComponentBeginOverlap(Sphere)
  (params (OverlappedComponent :type Primitive%20Component%20Object%20Reference) (OtherActor :type Actor%20Object%20Reference) (OtherComp :type Primitive%20Component%20Object%20Reference) (OtherBodyIndex :type Integer) (bFromSweep :type Boolean) (SweepResult :type Hit%20Result%20Structure%20%28by%20ref%29))
  (if (Math|Boolean|ANDBoolean (Actor|ActorHasTag OtherActor "Player") (> (Variables|Default|GetHealth) 0.0) true)
    (Game|Damage|ApplyDamage OtherActor 1e+01 0 0)))

(event EventBeginPlay
  (bind _mesh (Variables|Character|GetMesh))
  (bind _bonename (Variables|Default|GetBoneName))
  (Class|SkeletalMeshComponent|SetAllBodiesBelowSimulatePhysics _mesh _bonename true false)
  (Class|SkeletalMeshComponent|SetAllBodiesBelowPhysicsBlendWeight _mesh _bonename 2.0 true false))

(event Collision|EventActorBeginOverlap
  (params (OtherActor :type Actor%20Object%20Reference)))

(event EventTick
  (params (DeltaSeconds :type Float%20%28single-precision%29)))

(event Game|Damage|EventAnyDamage
  (params (Damage :type Float%20%28single-precision%29) (DamageType :type Damage%20Type%20Object%20Reference) (InstigatedBy :type Controller%20Object%20Reference) (DamageCauser :type Actor%20Object%20Reference))
  (Variables|Default|SetHealth (- (Variables|Default|GetHealth) Damage))
  (if (<= (Variables|Default|GetHealth) 0.0)
    (Utilities|FlowControl|DoOnce false
      (:Completed
        (Class|SkeletalMeshComponent|SetAllBodiesSimulatePhysics (Variables|Character|GetMesh) true)
        (Components|DestroyComponent (Variables|Collision|GetCapsuleComponent))
        (Math|Integer|IncrementInt (Variables|/Game/Blueprints/ZombieGameMode.ZombieGameMode_C|GetNumZombie (.AsZombie%20Game%20Mode (Utilities|Casting|CastToZombieGameMode (Game|GetGameMode))))
          (:%20%20
            (Actor|SetLifeSpan 3.0)))))))

(fn ConstructionScript
  (Variables|/Script/Engine.CharacterMovementComponent|SetMaxWalkSpeed (Variables|Character|GetCharacterMovement) (Variables|Default|GetSpeed)))
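; ZombieGameMode is a game mode Blueprint that runs the match timer and ends the game when time runs out.
; Tick accumulates elapsed time, clamps it at MaxTime and sets IsGameOver, then switches the first player controller to UI-only input with a visible cursor.
; The following tick sees the flag and disables further ticking.
; NumZombie appears only in an unconnected string conversion, so no zombie-count logic runs here.
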(event EventBeginPlay)

(event EventTick
  (params (DeltaSeconds :type Float%20%28single-precision%29))
  (bind _returnvalue (Game|GetPlayerController 0))
  (if (Variables|Default|GetIsGameOver)
    (Actor|Tick|SetActorTickEnabled self)
    (else
      (bind _output_get (Variables|Default|SetTime (+ DeltaSeconds (Variables|Default|GetTime))))
      (if (>= (Variables|Default|GetTime) (Variables|Default|GetMaxTime))
        (Variables|Default|SetTime (Variables|Default|GetMaxTime))
        (Variables|Default|SetIsGameOver true)
        (Input|SetInputModeUIOnly _returnvalue 0 "DoNotLock")
        (Variables|/Script/Engine.PlayerController|SetbShowMouseCursor _returnvalue true)))))

(fn ConstructionScript)